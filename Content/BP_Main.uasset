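; BP_Main is the actor that starts the game's main interface and exposes approval ratings for population groups, split by income, age, belief and other demographics.
; On BeginPlay it creates and displays WBP_Main, switches to UI-only input with a visible cursor, and plays background music.
; One getter per group reads a fixed index of the widget's ApprovalActuals array, so the approval values live in the UI.
; AddMediaWidget is an empty event.
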(event Custom|AddMediaWidget)

(event EventBeginPlay
  (bind _returnvalue (Game|GetPlayerController 0))
  (bind _returnvalue_2 (UserInterface|CreateWidget "/Game/WBP_Main.WBP_Main_C"))
  (bind _output_get (Variables|Default|SetInterface _returnvalue_2))
  (UserInterface|Viewport|AddtoViewport _output_get 1000)
  (Input|SetInputModeUIOnly _returnvalue _output_get "DoNotLock")
  (Variables|/Script/Engine.PlayerController|SetbShowMouseCursor _returnvalue true)
  (Audio|PlaySound2D "/Game/BackgroundMusic.BackgroundMusic"))

(event Collision|EventActorBeginOverlap
  (params (OtherActor :type Actor%20Object%20Reference)))

(event EventTick
  (params (DeltaSeconds :type Float%20%28single-precision%29)))

(fn ConstructionScript)

(fn LowIncomeApproval
  (return (Utilities|Array|Get(acopy) (Variables|/Game/WBP_Main.WBP_Main_C|GetApprovalActuals (Variables|Default|GetInterface)))))

(fn MiddleIncomeApproval
  (return (Utilities|Array|Get(acopy) (Variables|/Game/WBP_Main.WBP_Main_C|GetApprovalActuals (Variables|Default|GetInterface)) 1)))

(fn WealthyApproval
  (return (Utilities|Array|Get(acopy) (Variables|/Game/WBP_Main.WBP_Main_C|GetApprovalActuals (Variables|Default|GetInterface)) 2)))

(fn YouthApproval
  (return (Utilities|Array|Get(acopy) (Variables|/Game/WBP_Main.WBP_Main_C|GetApprovalActuals (Variables|Default|GetInterface)) 3)))

(fn RetiredApproval
  (return (Utilities|Array|Get(acopy) (Variables|/Game/WBP_Main.WBP_Main_C|GetApprovalActuals (Variables|Default|GetInterface)) 4)))

(fn MinoritiesApproval
  (return (Utilities|Array|Get(acopy) (Variables|/Game/WBP_Main.WBP_Main_C|GetApprovalActuals (Variables|Default|GetInterface)) 5)))

(fn PatriotApproval
  (return (Utilities|Array|Get(acopy) (Variables|/Game/WBP_Main.WBP_Main_C|GetApprovalActuals (Variables|Default|GetInterface)) 6)))

(fn ReligiousApproval
  (return (Utilities|Array|Get(acopy) (Variables|/Game/WBP_Main.WBP_Main_C|GetApprovalActuals (Variables|Default|GetInterface)) 7)))

(fn SocialistApproval
  (return (Utilities|Array|Get(acopy) (Variables|/Game/WBP_Main.WBP_Main_C|GetApprovalActuals (Variables|Default|GetInterface)) 8)))

(fn CapitalistApproval
  (return (Utilities|Array|Get(acopy) (Variables|/Game/WBP_Main.WBP_Main_C|GetApprovalActuals (Variables|Default|GetInterface)) 9)))

(fn WomenApproval
  (return (Utilities|Array|Get(acopy) (Variables|/Game/WBP_Main.WBP_Main_C|GetApprovalActuals (Variables|Default|GetInterface)) 10)))